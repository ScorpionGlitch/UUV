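; Character Blueprint that handles object interaction and a toggleable rifle, and runs the BT_PlayerAssist behavior tree through its AI controller on BeginPlay.
; InteractionBox overlaps track actors implementing I_Interactable, and the interact event messages the first one in range.
; EquipWeapon flips the ABP_Male rifle-holding flag, spawning CurrentWeapon on the RightHand socket or destroying it.
; Attack input plays a hip-fire montage while a weapon is held.
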(event `self.ReceiveBeginPlay`
  (`AIController.RunBehaviorTree` (`AIBlueprintHelperLibrary.GetAIController` self) "/Game/UUV/AI/PlayerAssist/BT_PlayerAssist.BT_PlayerAssist"))

(event `Interact With Object In Range`
  (message `/Game/UUV/Blueprints/Interfaces/I_Interactable.InteractWith` (`|GetArrayItem` (`self.InteractablesInRange`))))

(event `Equip Weapon`
  (bind _asabp_male (cast `/Game/UUV/Animations/Mannequin/Male/ABP_Male` (`SkeletalMeshComponent.GetAnimInstance` (`self.Mesh`))))
  (bind _output_get (set `/Game/UUV/Animations/Mannequin/Male/ABP_Male.IsHoldingRifle?` (not (`/Game/UUV/Animations/Mannequin/Male/ABP_Male.IsHoldingRifle?` _asabp_male)) _asabp_male))
  (if _output_get
    (bind _returnvalue (`|SpawnActorFromClass` (`self.CurrentWeapon`) (`KismetMathLibrary.MakeTransform` (0.0 0.0 0.0)) "Undefined" "OverrideRootScale" null null))
    (bind _output_get_2 (set `self.CurrentWeaponActor` _returnvalue))
    (`self.K2_AttachToComponent` _output_get_2 (`self.Mesh`) "RightHand" "KeepRelative" "KeepRelative" "KeepRelative" true)
    (else
      (`self.K2_DestroyActor` (`self.CurrentWeaponActor`)))))

(event `self.InteractionBox.OnComponentBeginOverlap`
  (params (OverlappedComponent :type "PrimitiveComponent Object Reference") (OtherActor :type "Actor Object Reference") (OtherComp :type "PrimitiveComponent Object Reference") (OtherBodyIndex :type Integer) (bFromSweep :type Boolean) (SweepResult :type "HitResult Structure (by ref)"))
  (if (`KismetSystemLibrary.DoesImplementInterface` OtherActor "/Game/UUV/Blueprints/Interfaces/I_Interactable.I_Interactable_C")
    (`KismetArrayLibrary.Array_AddUnique` (`self.InteractablesInRange`) OtherActor)))

(event `self.InteractionBox.OnComponentEndOverlap`
  (params (OverlappedComponent :type "PrimitiveComponent Object Reference") (OtherActor :type "Actor Object Reference") (OtherComp :type "PrimitiveComponent Object Reference") (OtherBodyIndex :type Integer))
  (`KismetArrayLibrary.Array_RemoveItem` (`self.InteractablesInRange`) OtherActor))

(event `InputAction|Attack`
  (params (Key :type "Key Structure"))
  (:`Pressed`
    (if (`KismetSystemLibrary.IsValid` (`self.CurrentWeaponActor`))
      (`self.PlayAnimMontage` "/Game/UUV/Animations/Mannequin/Male/Fire_Rifle_Hip_Montage.Fire_Rifle_Hip_Montage"))))

(fn `UserConstructionScript`)
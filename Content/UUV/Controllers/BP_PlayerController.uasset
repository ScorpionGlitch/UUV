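; Player controller that spawns and possesses the player character and handles switching between on-foot and vehicle states.
; To enter a vehicle, it hands the pawn to BP_PlayerAssistController and writes the target to its Blackboard.
; On reaching the door, it disables capsule collision, changes animation state and attaches the character to the Seat socket, without possessing the vehicle.
; ControlPlayer detaches and offsets the character, restores collision and animation, then repossesses it.
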(event `self.ReceiveBeginPlay`
  (bind _returnvalue (`|SpawnActorFromClass` "/Game/UUV/Characters/BP_PlayerCharacter.BP_PlayerCharacter_C" (`KismetMathLibrary.MakeTransform` (0.0 0.0 200.0) (struct :`Yaw` 180.0)) "Undefined" "OverrideRootScale" null null))
  (bind _output_get (set `self.PlayerPawn` _returnvalue))
  (set `self.PlayerAssist` (cast `/Game/UUV/Controllers/BP_PlayerAssistController` (`AIBlueprintHelperLibrary.GetAIController` _output_get) :!pure true))
  (`self.Possess` (`self.PlayerPawn`)))

(event `self.ReceivePossess`
  (params (PossessedPawn :type "Pawn Object Reference"))
  (if (not (`KismetSystemLibrary.IsValid` (`self.PlayerPawn`)))
    (bind _asbp_player_character (cast `/Game/UUV/Characters/BP_PlayerCharacter` PossessedPawn))
    (set `self.PlayerPawn` _asbp_player_character)))

(event `Event Control Player`
  (`self.UnPossess`)
  (`self.K2_DetachFromActor` (`self.PlayerPawn`) "KeepWorld" "KeepRelative" "KeepRelative")
  (set `/Game/UUV/Animations/Mannequin/Male/ABP_Male.CharacterState` "NewEnumerator0" (cast `/Game/UUV/Animations/Mannequin/Male/ABP_Male` (`SkeletalMeshComponent.GetAnimInstance` (`Character.Mesh` (`self.PlayerPawn`))) :!pure true))
  (`self.K2_AddActorLocalOffset` (`self.PlayerPawn`) (0.0 -100.0 50.0) false false)
  (`PrimitiveComponent.SetCollisionEnabled` (`Character.CapsuleComponent` (`self.PlayerPawn`)) "QueryAndPhysics")
  (`self.Possess` (`self.PlayerPawn`)))

(event `Event Attempt Control Vehicle`
  (params (Vehicle :type "/Game/UUV/Pawns/Sedan/Sedan Object Reference"))
  (bind _blackboard (`AIController.Blackboard` (`self.PlayerAssist`)))
  (`self.UnPossess`)
  (`self.Possess` (`self.PlayerAssist`) (`self.PlayerPawn`))
  (if (`KismetSystemLibrary.IsValid` _blackboard)
    (`BlackboardComponent.SetValueAsObject` _blackboard "VehicleToDrive" Vehicle)))

(event `Event Reached Vehicle Door`
  (params (Vehicle :type "/Game/UUV/Pawns/Sedan/Sedan Object Reference"))
  (`PrimitiveComponent.SetCollisionEnabled` (`Character.CapsuleComponent` (`self.PlayerPawn`)) "NoCollision")
  (set `/Game/UUV/Animations/Mannequin/Male/ABP_Male.CharacterState` "NewEnumerator2" (cast `/Game/UUV/Animations/Mannequin/Male/ABP_Male` (`SkeletalMeshComponent.GetAnimInstance` (`Character.Mesh` (`self.PlayerPawn`))) :!pure true))
  (`self.K2_AttachToActor` (`self.PlayerPawn`) Vehicle "Seat" "SnapToTarget" "SnapToTarget" "KeepWorld" false))

(fn `ControlPlayer`
  (`self.UnPossess`)
  (`self.K2_DetachFromActor` (`self.PlayerPawn`) "KeepWorld" "KeepRelative" "KeepRelative")
  (set `/Game/UUV/Animations/Mannequin/Male/ABP_Male.CharacterState` "NewEnumerator0" (cast `/Game/UUV/Animations/Mannequin/Male/ABP_Male` (`SkeletalMeshComponent.GetAnimInstance` (`Character.Mesh` (`self.PlayerPawn`))) :!pure true))
  (`self.K2_AddActorLocalOffset` (`self.PlayerPawn`) (0.0 -100.0 50.0) false false)
  (`PrimitiveComponent.SetCollisionEnabled` (`Character.CapsuleComponent` (`self.PlayerPawn`)) "QueryAndPhysics")
  (`self.Possess` (`self.PlayerPawn`)))

(fn `UserConstructionScript`)